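; Shopper AI pawn that wanders between random waypoints and hops as it goes.
; After a startup delay, it finds TrollyGameMode_BP via GetAllActorsOfClass and issues AIMoveTo toward a random WayArray entry.
; Straight after issuing the move, without waiting for arrival, it applies an upward velocity impulse to its root primitive, then loops after a random whole-second delay to pick a new target.
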(event `self.ReceiveBeginPlay`
  (`KismetSystemLibrary.Delay` 5.0)
  (bind _outactors (`GameplayStatics.GetAllActorsOfClass` "/Game/Blueprints/TrollyGameMode_BP.TrollyGameMode_BP_C" :!label _label))
  (bind _wayarray (`/Game/Blueprints/TrollyGameMode_BP.WayArray` (`KismetArrayLibrary.Array_Get` _outactors)))
  (`|AIMoveTo` self (0.0 0.0 0.0) (`KismetArrayLibrary.Array_Get` _wayarray (`KismetMathLibrary.RandomInteger` (`KismetArrayLibrary.Array_Length` _wayarray)))
    (:`then`
      (bind _asprimitive_component (cast `PrimitiveComponent` (`self.K2_GetRootComponent`)))
      (`PrimitiveComponent.AddImpulse` _asprimitive_component (0.0 0.0 300.0) "None" true)
      (`KismetSystemLibrary.Delay` (`KismetMathLibrary.Conv_IntToDouble` (`KismetMathLibrary.RandomInteger` 5)))
      (goto _label))))

(event `self.ReceiveTick`
  (params (DeltaSeconds :type "Float (single-precision)")))

(fn `UserConstructionScript`)