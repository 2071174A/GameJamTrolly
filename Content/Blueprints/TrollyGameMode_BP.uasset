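; TrollyGameMode_BP is the trolly level's game mode, which runs a timed round and opens ScoreMap when the countdown expires.
; BeginPlay plays a splash sound, creates the timer HUD and collects actors whose first tag is "Way" into WayArray.
; Tick accumulates elapsed time against the countdown.
; Custom events play a given sound and briefly set an Image variable before resetting it to transparent; the HUD alert event only looks up widgets.
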(event `self.ReceiveBeginPlay`
  (`self.CustomEventSound` "/Game/Sound/Trolly_Splash.Trolly_Splash")
  (set `self.CountdownTime` 60.0)
  (bind _returnvalue (`|CreateWidget` "/Game/Blueprints/TimerHUD.TimerHUD_C"))
  (`UserWidget.AddToViewport` _returnvalue 0)
  (bind _outactors (`GameplayStatics.GetAllActorsOfClass` "/Script/Engine.Actor"))
  (for _array_element _outactors
    (if (`KismetStringLibrary.EqualEqual_StrStr` (`KismetStringLibrary.Conv_NameToString` (`KismetArrayLibrary.Array_Get` (`Actor.Tags` _array_element))) "Way")
      (`KismetArrayLibrary.Array_Add` (`self.WayArray`) _array_element))))

(event `self.ReceiveTick`
  (params (DeltaSeconds :type "Float (single-precision)"))
  (bind _output_get (set `self.ElapsedTime` (+ (`self.ElapsedTime`) DeltaSeconds)))
  (if (> _output_get (`self.CountdownTime`))
    (`GameplayStatics.OpenLevel` "ScoreMap")))

(event `CustomEventSound`
  (params (NewParam :type "SoundWave Object Reference"))
  (`GameplayStatics.PlaySoundAtLocation` NewParam (`self.K2_GetActorLocation`)))

(event `CustomCreateAlert`
  (bind _foundwidgets (`WidgetBlueprintLibrary.GetAllWidgetsOfClass` "/Game/Blueprints/TimerHUD.TimerHUD_C")))

(event `CustomDisplayMessageImageToHud`
  (params (Image :type "Texture Object Reference"))
  (set `self.Image` Image)
  (`KismetSystemLibrary.Delay` 5.0)
  (set `self.Image` "/Game/Art/Output/transparent.transparent"))

(fn `UserConstructionScript`)